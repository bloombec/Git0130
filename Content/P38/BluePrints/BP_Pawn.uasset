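; BP_Pawn is a player-controlled P38 plane pawn that constantly moves forward and fires rockets.
; Tick applies forward movement input and spins the left and right propellers, scaled by delta seconds for frame-rate independence.
; BeginPlay adds the Enhanced Input mapping context, whose actions feed controller roll and pitch or spawn BP_Rocket at the Arrow's transform.
; The Pitch and Roll axis events are empty.
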(event Input|EnhancedActionEvents|EnhancedInputActionIA_Fire
  (params (ActionValue :type Boolean) (ElapsedSeconds :type Float%20%28double-precision%29) (TriggeredSeconds :type Float%20%28double-precision%29) (InputAction :type Input%20Action%20Object%20Reference :default "/Game/P38/BluePrints/Input/IA_Fire.IA_Fire"))
  ;[1 1 1] 입력값 설정하고 미사일 발사
  (:Triggered
    (Game|SpawnActorfromClass "/Game/P38/BluePrints/BP_Rocket.BP_Rocket_C" (Transformation|GetWorldTransform (Variables|Default|GetArrow)) "Undefined" 0 0)))

(event Input|EnhancedActionEvents|EnhancedInputActionIA_PitchAndRoll
  (params (ActionValue :type Vector%202D%20Structure) (ElapsedSeconds :type Float%20%28double-precision%29) (TriggeredSeconds :type Float%20%28double-precision%29) (InputAction :type Input%20Action%20Object%20Reference :default "/Game/P38/BluePrints/Input/IA_PitchAndRoll.IA_PitchAndRoll"))
  (:Triggered
    (Pawn|Input|AddControllerRollInput (.x ActionValue))
    (Pawn|Input|AddControllerPitchInput (.y ActionValue))))

(event EventBeginPlay
  (Utilities|IsValid (Game|GetPlayerController 0)
    (:Is%20Valid
      (Input|AddMappingContext (PlayerController|LocalPlayerSubsystems|GetEnhancedInputLocalPlayerSubsystem (Game|GetPlayerController 0)) "/Game/P38/BluePrints/Input/IMC_Input.IMC_Input" 0 "(bIgnoreAllPressedKeysUntilRelease=True,bForceImmediately=False)"))))

(event EventTick
  (params (DeltaSeconds :type Float%20%28single-precision%29))
  ;[1 1 1] 이동
  (Pawn|Input|AddMovementInput (Transformation|GetActorForwardVector) 1.0 false)
  ;[1 1 1] 시간을 통일해주기 위해서 델타세컨즈 함수 가져옴
  ;;[1 1 1] 한 프레임당 10도 회전: 컴퓨터 사양마다 걸리는 시간이 다르니까
  (Transformation|AddLocalRotation (Variables|Default|GetLeft) (* (Variables|Default|GetPropellerRotationSpeed) (Utilities|Time|GetWorldDeltaSeconds)) false false)
  ;[1 1 1] 왼쪽, 오른쪽 프로펠러 회전
  (Transformation|AddLocalRotation (Variables|Default|GetRight) (* (Variables|Default|GetPropellerRotationSpeed) (Utilities|Time|GetWorldDeltaSeconds)) false false))

(event Input|ActionEvents|InputActionFire
  (params (Key :type Key%20Structure :default "None"))
  ;[1 1 1] 입력값 설정하고 미사일 발사
)

(event Input|AxisEvents|InputAxisPitch
  (params (AxisValue :type Float%20%28single-precision%29)))

(event Input|AxisEvents|InputAxisRoll
  (params (AxisValue :type Float%20%28single-precision%29)))

(fn ConstructionScript)