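; BP_P38 is a P-38 plane Blueprint built to spin its two propellers and move forward along local X.
; RotatePropeller rolls a given propeller component by RotationSpeed scaled by frame delta time.
; The calls for both propellers and the MoveSpeed-based actor offset are disconnected from any event, and Tick is empty, so the plane neither moves nor animates as wired.
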(event EventTick
  (params (DeltaSeconds :type Float%20%28single-precision%29)))

(fn ConstructionScript)

(fn RotatePropeller
  (params (Where :type Scene%20Component%20Object%20Reference))
  (Transformation|AddLocalRotation Where (Math|Rotator|MakeRotator (* (Variables|속력|GetRotationSpeed) (Utilities|Time|GetWorldDeltaSeconds)) 0.0 0.0) false false))